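; Goal actor (Meta) that hides its mesh until the player's score (Puntos) reaches 15, then acts as the victory trigger.
; Tick polls the score and, through a DoOnce, reveals the mesh and opens a Gate fed by any Box overlap.
; Passing the Gate disables input, pauses the game, shows a fade and PauseMenu's second page, and swaps music and lava audio for victory audio.
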(event `self.ReceiveBeginPlay`
  (`SceneComponent.SetVisibility` (`self.StaticMeshComponent`) false true))

(event `self.ReceiveTick`
  (params (DeltaSeconds :type "Float (single-precision)"))
  (bind _returnvalue (`GameplayStatics.GetPlayerController` 0))
  (bind _asfirst_person_character (cast `/Game/Blueprints/Characters/FirstPersonCharacter/FirstPersonCharacter` (`GameplayStatics.GetPlayerCharacter` 0) :!pure true))
  (if (>= (`/Game/Blueprints/Characters/FirstPersonCharacter/FirstPersonCharacter.puntos` (cast `/Game/Blueprints/Characters/FirstPersonCharacter/FirstPersonCharacter` (`GameplayStatics.GetPlayerCharacter` 0) :!pure true)) 15)
    (`/Engine/EditorBlueprintResources/StandardMacros.DoOnce` false
      (:`Completed`
        (`SceneComponent.SetVisibility` (`self.StaticMeshComponent`) true true)
        (goto _label :!via `Open`)))))

(event `self.Box.OnComponentBeginOverlap`
  (params (OverlappedComponent :type "PrimitiveComponent Object Reference") (OtherActor :type "Actor Object Reference") (OtherComp :type "PrimitiveComponent Object Reference") (OtherBodyIndex :type Integer) (bFromSweep :type Boolean) (SweepResult :type "HitResult Structure (by ref)"))
  (bind _returnvalue (`GameplayStatics.GetPlayerController` 0))
  (bind _asfirst_person_character (cast `/Game/Blueprints/Characters/FirstPersonCharacter/FirstPersonCharacter` (`GameplayStatics.GetPlayerCharacter` 0) :!pure true))
  (`/Engine/EditorBlueprintResources/StandardMacros.Gate` true :!label _label
    (:`Exit`
      (`self.DisableInput` (`GameplayStatics.GetPlayerController` 0))
      (`UserWidget.AddToViewport` (`self.WidgetFade`) 0)
      (`KismetSystemLibrary.K2_ClearTimer` null "refreshStopwatch")
      (`GameplayStatics.SetGamePaused` true)
      (bind _returnvalue_2 (`|CreateWidget` "/Game/Blueprints/Widgets/Menu/PauseMenu.PauseMenu_C"))
      (`UserWidget.AddToViewport` _returnvalue_2 0)
      (`WidgetSwitcher.SetActiveWidgetIndex` (`/Game/Blueprints/Widgets/Menu/PauseMenu.WidgetSwitcher_201` _returnvalue_2) 1)
      (`AudioComponent.Stop` (`/Game/Blueprints/Characters/FirstPersonCharacter/FirstPersonCharacter.Musicafondo` _asfirst_person_character))
      (`AudioComponent.Stop` (`/Game/Blueprints/Characters/FirstPersonCharacter/FirstPersonCharacter.Sonido Lava` _asfirst_person_character))
      (`AudioComponent.Play` (`self.Victoria`) 0.0)
      (`WidgetBlueprintLibrary.SetInputMode_UIOnlyEx` _returnvalue _returnvalue_2)
      (set `PlayerController.bShowMouseCursor` true _returnvalue))))

(fn `UserConstructionScript`)