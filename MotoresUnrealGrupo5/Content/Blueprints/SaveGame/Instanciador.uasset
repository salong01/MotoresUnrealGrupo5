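; Instanciador saves and loads the player's position through GuardarInfo save objects.
; GuardarPartida reuses or creates a save, stores the pawn transform, and writes it to a slot named after the current level.
; CargarPartida reads from SlotName, opens the stored Level, then applies the transform after a 0.2-second delay.
; Saving never sets the Level field, and its write slot differs from the SlotName variable used for reads.
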(event `CargarPartida`
  (bind _returnvalue (`GameplayStatics.LoadGameFromSlot` (`self.Slot Name`)))
  (bind _asguardar_info (cast `/Game/Blueprints/SaveGame/GuardarInfo` _returnvalue))
  (bind _output_get (set `self.PoisicionJugador` (`/Game/Blueprints/SaveGame/GuardarInfo.Posicion` _asguardar_info)))
  (`GameplayStatics.OpenLevel` (`KismetStringLibrary.Conv_StringToName` (`/Game/Blueprints/SaveGame/GuardarInfo.Level` _asguardar_info)))
  (`KismetSystemLibrary.Delay` 0.2)
  (`Actor.K2_SetActorTransform` (`GameplayStatics.GetPlayerPawn` 0) _output_get false false))

(event `GuardarPartida`
  (bind _slot_name (`self.Slot Name`))
  (bind _nivel (`self.Nivel`))
  (bind _returnvalue (`Actor.GetTransform` (`GameplayStatics.GetPlayerPawn` 0)))
  (bind _returnvalue_2 (`GameplayStatics.DoesSaveGameExist` _slot_name))
  (if _returnvalue_2
    (bind _returnvalue_3 (`GameplayStatics.LoadGameFromSlot` _slot_name))
    (bind _asguardar_info (cast `/Game/Blueprints/SaveGame/GuardarInfo` _returnvalue_3))
    (set `/Game/Blueprints/SaveGame/GuardarInfo.Posicion` _returnvalue _asguardar_info)
    (bind _returnvalue_4 (`GameplayStatics.GetCurrentLevelName` true))
    (set `self.Nivel` _returnvalue_4)
    (`GameplayStatics.SaveGameToSlot` _returnvalue_3 _nivel)
    (else
      (bind _returnvalue_5 (`GameplayStatics.CreateSaveGameObject` "/Game/Blueprints/SaveGame/GuardarInfo.GuardarInfo_C"))
      (set `/Game/Blueprints/SaveGame/GuardarInfo.Posicion` _returnvalue _returnvalue_5)
      (bind _returnvalue_6 (`GameplayStatics.GetCurrentLevelName` true))
      (set `self.Nivel` _returnvalue_6)
      (`GameplayStatics.SaveGameToSlot` _returnvalue_5 _nivel))))