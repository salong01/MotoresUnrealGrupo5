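; LavaController is a pressure-plate trigger that moves a referenced Lava actor vertically when the first-person character steps on it.
; Box overlap sinks the Cube and actor end overlap restores it, with two DoOnce nodes resetting each other to alternate these states.
; Each box overlap also re-captures the lava's location and restarts the Movement timeline, which lerps its world Z to LavaHeight's Z.
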(event `self.ReceiveActorEndOverlap`
  (params (OtherActor :type "Actor Object Reference"))
  (cast `/Game/Blueprints/Characters/FirstPersonCharacter/FirstPersonCharacter` OtherActor)
  (`/Engine/EditorBlueprintResources/StandardMacros.DoOnce` false :!label _label
    (:`Completed`
      (`SceneComponent.K2_SetRelativeLocation` (`self.Cube`) (0.0 0.0 0.0) false false)
      (goto _label_2 :!via `Reset`))))

(event `self.Box.OnComponentBeginOverlap`
  (params (OverlappedComponent :type "PrimitiveComponent Object Reference") (OtherActor :type "Actor Object Reference") (OtherComp :type "PrimitiveComponent Object Reference") (OtherBodyIndex :type Integer) (bFromSweep :type Boolean) (SweepResult :type "HitResult Structure (by ref)"))
  (bind (_lavaheight_x _lavaheight_y _lavaheight_z) (`KismetMathLibrary.BreakVector` (`self.LavaHeight`)))
  (bind (_initiallocation_x _initiallocation_y _initiallocation_z) (`KismetMathLibrary.BreakVector` (`self.InitialLocation`)))
  (bind _returnvalue_location (`KismetMathLibrary.BreakTransform` (`SceneComponent.K2_GetComponentToWorld` (`Actor.RootComponent` (`self.Lava`)))))
  (cast `/Game/Blueprints/Characters/FirstPersonCharacter/FirstPersonCharacter` OtherActor)
  (`|ExecutionSequence`
    (:`then_0`
      (`/Engine/EditorBlueprintResources/StandardMacros.DoOnce` false :!label _label_2
        (:`Completed`
          (`SceneComponent.K2_SetRelativeLocation` (`self.Cube`) (0.0 0.0 -8.0) false false)
          (goto _label :!via `Reset`))))
    (:`then_1`
      (set `self.InitialLocation` _returnvalue_location)
      (bind (_direction _alpha) (`Timeline|Movement` :!via `PlayFromStart`)
        (:`Update`
          (`SceneComponent.K2_SetWorldLocation` (`Actor.RootComponent` (`self.Lava`)) (`KismetMathLibrary.MakeVector` _initiallocation_x _initiallocation_y (`KismetMathLibrary.Lerp` _initiallocation_z _lavaheight_z _alpha)) false false))))))

(fn `UserConstructionScript`
  (bind _returnvalue_location (`KismetMathLibrary.BreakTransform` (`SceneComponent.K2_GetComponentToWorld` (`Actor.RootComponent` (`self.Lava`)))))
  (set `self.InitialLocation` _returnvalue_location))