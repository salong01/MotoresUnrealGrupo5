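; Destructible button platform that floats at lava height along a spline and destroys itself shortly after its travel time expires.
; Timelines drive spline position, vertical bobbing relative to the lava, and yaw between two random angles chosen at construction.
; When the first-person character enters the box, the button depresses and a timeline moves the lava toward a target height.
; DoOnce nodes reset each other to toggle the button as the player enters and leaves.
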(event `self.ReceiveActorEndOverlap`
  (params (OtherActor :type "Actor Object Reference"))
  (cast `/Game/Blueprints/Characters/FirstPersonCharacter/FirstPersonCharacter` OtherActor)
  (`/Engine/EditorBlueprintResources/StandardMacros.DoOnce` false :!label _label
    (:`Completed`
      (`SceneComponent.K2_SetRelativeLocation` (`self.Button`) (0.0 0.0 0.0) false false)
      (goto _label_2 :!via `Reset`))))

(event `self.Box.OnComponentBeginOverlap`
  (params (OverlappedComponent :type "PrimitiveComponent Object Reference") (OtherActor :type "Actor Object Reference") (OtherComp :type "PrimitiveComponent Object Reference") (OtherBodyIndex :type Integer) (bFromSweep :type Boolean) (SweepResult :type "HitResult Structure (by ref)"))
  (bind (_lavaheight_x _lavaheight_y _lavaheight_z) (`KismetMathLibrary.BreakVector` (`self.LavaHeight`)))
  (bind (_initiallocation_x _initiallocation_y _initiallocation_z) (`KismetMathLibrary.BreakVector` (`self.InitialLocation`)))
  (bind _returnvalue_location (`KismetMathLibrary.BreakTransform` (`SceneComponent.K2_GetComponentToWorld` (`Actor.RootComponent` (`self.Lava`)))))
  (cast `/Game/Blueprints/Characters/FirstPersonCharacter/FirstPersonCharacter` OtherActor)
  (`|ExecutionSequence`
    (:`then_0`
      (`/Engine/EditorBlueprintResources/StandardMacros.DoOnce` false :!label _label_2
        (:`Completed`
          (`SceneComponent.K2_SetRelativeLocation` (`self.Button`) (0.0 0.0 -8.0) false false)
          (goto _label :!via `Reset`))))
    (:`then_1`
      (set `self.InitialLocation` _returnvalue_location)
      (bind (_direction _alpha) (`Timeline|Timeline` :!via `PlayFromStart`)
        (:`Update`
          (`SceneComponent.K2_SetWorldLocation` (`Actor.RootComponent` (`self.Lava`)) (`KismetMathLibrary.MakeVector` _initiallocation_x _initiallocation_y (`KismetMathLibrary.Lerp` _initiallocation_z _lavaheight_z _alpha)) false false))))))

(event `self.ReceiveBeginPlay`
  (bind _spline (`/Game/Blueprints/Platforms/SplinePath.Spline` (`self.SplinePath`)))
  (bind _returnvalue_location (`KismetMathLibrary.BreakTransform` (`SceneComponent.K2_GetComponentToWorld` (`Actor.RootComponent` (`self.Lava`)))))
  (`KismetSystemLibrary.Delay` 0.1)
  (set `self.InitialLocation` _returnvalue_location)
  (`|ExecutionSequence`
    (:`then_0`
      (`KismetSystemLibrary.Delay` (+ (`self.TimeToComplete`) 2.0))
      (`self.K2_DestroyActor`))
    (:`then_1`
      (`TimelineComponent.SetPlayRate` (`self.Movement`) (/ 1.0 (`self.TimeToComplete`)))
      (`TimelineComponent.SetPlayRate` (`self.FloatingMovement`) (/ 1.0 (`self.TimeToComplete`)))
      (bind (_direction _alpha) (`Timeline|Movement`)
        (:`Update`
          (`Timeline|Rotation` :!via `PlayFromStart`
            (:`Update`
              (bind (_direction_2 _floatz) (`Timeline|FloatingMovement`)
                (:`Update`
                  (bind (_returnvalue_x _returnvalue_y) (`KismetMathLibrary.BreakVector` (`SplineComponent.GetLocationAtDistanceAlongSpline` _spline (`KismetMathLibrary.Lerp` 0.0 (`SplineComponent.GetSplineLength` _spline) _alpha) "World")))
                  (`self.K2_SetActorTransform` (`KismetMathLibrary.MakeTransform` (`KismetMathLibrary.MakeVector` _returnvalue_x _returnvalue_y (+ (.z (.location (`self.GetTransform` (`self.Lava`)))) _floatz)) (`KismetMathLibrary.MakeRotator` 0.0 0.0 (`KismetMathLibrary.Lerp` (`self.Rot1`) (`self.Rot2`) _alpha)))))))))))))

(fn `UserConstructionScript`
  (set `self.InitialTransform` (`self.GetTransform`))
  (set `self.Rot1` (`KismetMathLibrary.RandomFloatInRange` -300.0 300.0))
  (set `self.Rot2` (`KismetMathLibrary.RandomFloatInRange` -300.0 300.0)))