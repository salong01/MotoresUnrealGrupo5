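; Geyser platform Blueprint whose column rises and falls in height on a timeline, starting at BeginPlay when Active or restarting through Activate.
; The timeline's Alpha moves an Arrow between minimum and maximum height and scales the geyser pivot to match, narrowing it as it grows taller.
; The construction script previews GeiserHeight, derives MaxHeight from the Arrow and sets playback speed; BeginPlay applies the start time offset and looping.
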(event `self.ReceiveBeginPlay`
  (`TimelineComponent.SetNewTime` (`self.GeiserAnimation`) (`self.Delay`))
  (`TimelineComponent.SetLooping` (`self.GeiserAnimation`) (`self.Looping`))
  (if (`self.Active`)
    (bind (_direction _alpha) (`Timeline|GeiserAnimation` :!label _label)
      (:`Update`
        (`SceneComponent.K2_SetRelativeLocation` (`self.Arrow`) (`KismetMathLibrary.VLerp` (`KismetMathLibrary.MakeVector` 0.0 0.0 (`self.MinHeight`)) (`KismetMathLibrary.MakeVector` 0.0 0.0 (`self.MaxHeight`)) _alpha) false false)
        (`SceneComponent.SetRelativeScale3D` (`self.PivotGeiser`) (`KismetMathLibrary.VLerp` (`KismetMathLibrary.MakeVector` 1.5 1.5 (/ (`self.MinHeight`) 100.0)) (`KismetMathLibrary.MakeVector` 0.8 0.8 (/ (`self.MaxHeight`) 100.0)) _alpha))))))

(event `Activate`
  (goto _label :!via `PlayFromStart`))

(fn `UserConstructionScript`
  (bind (_relativelocation_x _relativelocation_y _relativelocation_z) (`KismetMathLibrary.BreakVector` (`SceneComponent.RelativeLocation` (`self.Arrow`))))
  (`SceneComponent.K2_SetRelativeLocation` (`self.Arrow`) (`KismetMathLibrary.MakeVector` 0.0 0.0 (`self.GeiserHeight`)) false false)
  (`SceneComponent.SetRelativeScale3D` (`self.PivotGeiser`) (`KismetMathLibrary.MakeVector` 1.0 1.0 (/ (`self.GeiserHeight`) 100.0)))
  (set `self.MaxHeight` _relativelocation_z)
  (`TimelineComponent.SetPlayRate` (`self.GeiserAnimation`) (`self.GeiserSpeed`)))