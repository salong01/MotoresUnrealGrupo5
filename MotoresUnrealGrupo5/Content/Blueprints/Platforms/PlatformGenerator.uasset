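; Generator actor that endlessly spawns moving lava-level platforms at its Arrow component's location.
; On BeginPlay it spawns the configured PlatformType, then repeats after a random delay of a few seconds.
; Each spawn is cast to PlataformaDestruible or PlataformaDestruibleBoton and receives the spline path, lava reference and travel time, with the button variant also getting lava height.
; The loop stops if the spawn matches neither class.
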(event `self.ReceiveBeginPlay`
  (bind _lava (`self.Lava`))
  (bind _splinepath (`self.SplinePath`))
  (bind _timetocomplete (`self.TimeToComplete`))
  (bind _returnvalue (`|SpawnActorFromClass` (`self.PlatformType`) (`KismetMathLibrary.MakeTransform` (`SceneComponent.K2_GetComponentLocation` (`self.Arrow`)) (`KismetMathLibrary.MakeRotator` 0.0)) "Undefined" "MultiplyWithRoot" null null :!label _label))
  (bind _asplataforma_destruible (cast `/Game/Blueprints/Platforms/PlataformaDestruible` _returnvalue)
    (:`then`
      (set `/Game/Blueprints/Platforms/PlataformaDestruible.SplinePath` _splinepath _asplataforma_destruible)
      (set `/Game/Blueprints/Platforms/PlataformaDestruible.Lava` _lava _asplataforma_destruible)
      (set `/Game/Blueprints/Platforms/PlataformaDestruible.TimeToComplete` _timetocomplete _asplataforma_destruible))
    (:`CastFailed`
      (bind _asplataforma_destruible_boton (cast `/Game/Blueprints/Platforms/PlataformaDestruibleBoton` _returnvalue))
      (set `/Game/Blueprints/Platforms/PlataformaDestruibleBoton.SplinePath` _splinepath _asplataforma_destruible_boton)
      (set `/Game/Blueprints/Platforms/PlataformaDestruibleBoton.Lava` _lava _asplataforma_destruible_boton)
      (set `/Game/Blueprints/Platforms/PlataformaDestruibleBoton.TimeToComplete` _timetocomplete _asplataforma_destruible_boton)
      (set `/Game/Blueprints/Platforms/PlataformaDestruibleBoton.LavaHeight` (`self.LavaHeight`) _asplataforma_destruible_boton)))
  (`KismetSystemLibrary.Delay` (`KismetMathLibrary.RandomFloatInRange` 2.5 4.5))
  (goto _label))

(fn `UserConstructionScript`)