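; PlataformaDestruible is a temporary platform that travels along a spline while bobbing relative to the lava's height, then destroys itself.
; Nested timelines drive the transform: Movement sets XY along SplinePath, while FloatingMovement adds a Z offset to the Lava actor's height.
; Yaw blends between two random angles chosen in the construction script, using Movement's alpha.
; TimeToComplete scales the Movement and FloatingMovement play rates and sets the delay before destruction.
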(event `self.ReceiveBeginPlay`
  (bind _spline (`/Game/Blueprints/Platforms/SplinePath.Spline` (`self.SplinePath`)))
  (`KismetSystemLibrary.Delay` 0.1)
  (`|ExecutionSequence`
    (:`then_0`
      (`KismetSystemLibrary.Delay` (+ (`self.TimeToComplete`) 2.0))
      (`self.K2_DestroyActor`))
    (:`then_1`
      (`TimelineComponent.SetPlayRate` (`self.Movement`) (/ 1.0 (`self.TimeToComplete`)))
      (`TimelineComponent.SetPlayRate` (`self.FloatingMovement`) (/ 1.0 (`self.TimeToComplete`)))
      (bind (_direction _alpha) (`Timeline|Movement`)
        (:`Update`
          (`Timeline|Rotation` :!via `PlayFromStart`
            (:`Update`
              (bind (_direction_2 _floatz) (`Timeline|FloatingMovement`)
                (:`Update`
                  (bind (_returnvalue_x _returnvalue_y) (`KismetMathLibrary.BreakVector` (`SplineComponent.GetLocationAtDistanceAlongSpline` _spline (`KismetMathLibrary.Lerp` 0.0 (`SplineComponent.GetSplineLength` _spline) _alpha) "World")))
                  (`self.K2_SetActorTransform` (`KismetMathLibrary.MakeTransform` (`KismetMathLibrary.MakeVector` _returnvalue_x _returnvalue_y (+ (.z (.location (`self.GetTransform` (`self.Lava`)))) _floatz)) (`KismetMathLibrary.MakeRotator` 0.0 0.0 (`KismetMathLibrary.Lerp` (`self.Rot1`) (`self.Rot2`) _alpha)))))))))))))

(fn `UserConstructionScript`
  (set `self.InitialTransform` (`self.GetTransform`))
  (set `self.Rot1` (`KismetMathLibrary.RandomFloatInRange` -300.0 300.0))
  (set `self.Rot2` (`KismetMathLibrary.RandomFloatInRange` -300.0 300.0)))